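; BP_Beacon is a hold-to-interact beacon light that the player disables.
; It builds on parent interaction logic, showing or hiding a WBP_InteractDisplay widget as interaction is offered or withdrawn.
; While pressed, Tick feeds hold-time progress into the widget's fill, which resets on release or hide.
; On success it hides the mesh and beam and destroys the widget component.
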(event `self.ReceiveBeginPlay`
  (`parent.ReceiveBeginPlay`)
  (`SceneComponent.SetVisibility` (`self.FillWidget`) false false)
  (bind _aswbp_interact_display (cast `/Game/ShadowStep/UI/Player/InteractButton/WBP_InteractDisplay` (`WidgetComponent.GetWidget` (`self.FillWidget`))))
  (bind _output_get (set `self.As WBP Interact Display` _aswbp_interact_display))
  (set `/Game/ShadowStep/UI/Player/InteractButton/WBP_InteractDisplay.ProgressValue` 0.0 _output_get))

(event `self.ReceiveTick`
  (params (DeltaSeconds :type "Float (single-precision)"))
  (`parent.ReceiveTick` DeltaSeconds)
  (if (`self.IsPressed`)
    (bind _holdtimeprogress (`self.GetHoldTimeProgress`))
    (`/Game/ShadowStep/UI/Player/InteractButton/WBP_InteractDisplay.SetFill` (`self.As WBP Interact Display`) _holdtimeprogress)))

(event `/Game/Development/Justin/Interface/BPI_Interactable.HideInteraction`
  (bind _fillwidget (`self.FillWidget`))
  ; Hide Light Disable Icon
  (`/Engine/EditorBlueprintResources/StandardMacros.IsValid` _fillwidget
    (:`Is Valid`
      (`SceneComponent.SetVisibility` _fillwidget false false)
      (`/Game/ShadowStep/UI/Player/InteractButton/WBP_InteractDisplay.SetFill` (`self.As WBP Interact Display`) 0.0))))

(event `/Game/Development/Justin/Interface/BPI_Interactable.ShowInteraction`
  (bind _fillwidget (`self.FillWidget`))
  ; Show Light Disable Icon
  (`/Engine/EditorBlueprintResources/StandardMacros.IsValid` _fillwidget
    (:`Is Valid`
      (`SceneComponent.SetVisibility` _fillwidget true false))))

(event `/Game/Development/Justin/Interface/BPI_Interactable.InteractStarted`
  (`parent.InteractStarted`)
  (set `self.IsPressed` true))

(event `/Game/Development/Justin/Interface/BPI_Interactable.InteractEnded`
  (`parent.InteractEnded`)
  (set `self.IsPressed` false)
  (`/Game/ShadowStep/UI/Player/InteractButton/WBP_InteractDisplay.SetFill` (`self.As WBP Interact Display`) 0.0))

(fn `OnInteractionSuccess`
  (`parent.OnInteractionSuccess`)
  ; Beacon Disapear
  (`SceneComponent.SetVisibility` (`self.InteractableMesh`) false false)
  (`SceneComponent.SetVisibility` (`self.BeaconBeam`) false false)
  (`ActorComponent.K2_DestroyComponent` (`self.FillWidget`)))

(fn `UserConstructionScript`
  (`parent.UserConstructionScript`))