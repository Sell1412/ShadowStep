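; Checkpoint actor that sets the player's respawn spot and can mark the transition into a new play area.
; It registers with BP_WorldGameMode on BeginPlay and submits itself as the new checkpoint when the player overlaps its trigger.
; With ShouldLoadNewArea set, it updates the current area and GoalManager, fires OnNewAreaLoad and turns any BlockingVolume into an invisible wall.
; GetRespawnLocation exposes the RespawnPoint's world transform.
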(event `self.ReceiveBeginPlay`
  (bind _asbp_world_game_mode (cast `/Game/ShadowStep/Core/ProjectManagers/BP_WorldGameMode` (`GameplayStatics.GetGameMode`)))
  (bind _output_get (set `self.Gamemode` _asbp_world_game_mode))
  (`/Game/ShadowStep/Core/ProjectManagers/BP_WorldGameMode.RegisterCheckpoint` _output_get self))

(event `self.EnterAreaTrigger.OnComponentBeginOverlap`
  (params (OverlappedComponent :type "PrimitiveComponent Object Reference") (OtherActor :type "Actor Object Reference") (OtherComp :type "PrimitiveComponent Object Reference") (OtherBodyIndex :type Integer) (bFromSweep :type Boolean) (SweepResult :type "HitResult Structure (by ref)"))
  (bind _blockingvolume (`self.BlockingVolume`))
  ; Player enters Area
  (cast `/Game/ShadowStep/Characters/Player/BP_PlayerCharakter` OtherActor)
  (`self.SetNewCheckpoint`)
  (if (`self.bShouldLoadNewArea`)
    (set `/Game/ShadowStep/Core/ProjectManagers/BP_WorldGameMode.CurrentPlayArea` (`self.NewArea`) (`self.Gamemode`))
    (`self.OnNewAreaLoad` self)
    (`/Game/ShadowStep/Core/ProjectManagers/Managers/BP_GoalManager.UpdateNewArea` (`/Game/ShadowStep/Core/ProjectManagers/BP_WorldGameMode.GoalManager` (`self.Gamemode`)))
    (`/Engine/EditorBlueprintResources/StandardMacros.IsValid` _blockingvolume
      (:`Is Valid`
        (`PrimitiveComponent.SetCollisionProfileName` (`Brush.BrushComponent` _blockingvolume) "InvisibleWall" true)))))

(fn `GetRespawnLocation`
  (returns (RespawnLocation :type "Transform Structure"))
  (return (`SceneComponent.K2_GetComponentToWorld` (`self.RespawnPoint`))))

(fn `SetNewCheckpoint`
  (bind _asbp_world_game_mode (cast `/Game/ShadowStep/Core/ProjectManagers/BP_WorldGameMode` (`GameplayStatics.GetGameMode`)))
  (bind _sucessfull (`/Game/ShadowStep/Core/ProjectManagers/BP_WorldGameMode.SetNewCheckpoint` _asbp_world_game_mode self))
  (if _sucessfull
    _))

(fn `UserConstructionScript`)