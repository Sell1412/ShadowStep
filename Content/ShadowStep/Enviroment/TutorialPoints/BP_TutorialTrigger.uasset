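; BP_TutorialTrigger is a tutorial point that shows upper and lower text on the player HUD for a set duration.
; It fires on BeginPlay when ShouldDisplayOnStart is set, or on any overlap with its Box, with both paths sharing one DoOnce.
; It casts the first player's HUD to BP_PlayerHUD, briefly delays if the HUD widget is invalid, and calls ShowTutoiral.
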(event `self.ReceiveBeginPlay`
  (if (`self.ShouldDisplayOnStart`)
    (`/Engine/EditorBlueprintResources/StandardMacros.DoOnce` false :!label _label
      (:`Completed`
        (bind _asbp_player_hud (cast `/Game/ShadowStep/Core/ProjectManagers/BP_PlayerHUD` (`PlayerController.GetHUD` (`GameplayStatics.GetPlayerController` 0))))
        (`/Engine/EditorBlueprintResources/StandardMacros.IsValid` (`/Game/ShadowStep/Core/ProjectManagers/BP_PlayerHUD.PlayerHudWidget` _asbp_player_hud)
          (:`Is Valid`
            _)
          (:`Is Not Valid`
            (`KismetSystemLibrary.Delay` 0.2)))
        (`/Game/ShadowStep/Core/ProjectManagers/BP_PlayerHUD.ShowTutoiral` _asbp_player_hud (`self.TutorialText_Upper`) (`self.TutorialText_Lower`) (`self.TutorialDisplayDuration`))))))

(event `self.ReceiveActorBeginOverlap`
  (params (OtherActor :type "Actor Object Reference")))

(event `self.Box.OnComponentBeginOverlap`
  (params (OverlappedComponent :type "PrimitiveComponent Object Reference") (OtherActor :type "Actor Object Reference") (OtherComp :type "PrimitiveComponent Object Reference") (OtherBodyIndex :type Integer) (bFromSweep :type Boolean) (SweepResult :type "HitResult Structure (by ref)"))
  (goto _label))

(fn `UserConstructionScript`)