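; AC_AreaControl is an actor component that puts its owning AI pawn to sleep or wakes it, apparently as part of area-based activation.
; ActivateArea and DeactivateArea toggle the AIC_BaseController pause flag, controller and owner tick, and the behavior logic on the controller's brain component.
; For Character owners they also switch mesh animation on or off.
; Both functions do nothing if the owner's controller is not an AIC_BaseController.
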(fn `ActivateArea`
  (bind _returnvalue (`self.GetOwner`))
  (bind _returnvalue_2 (`AIBlueprintHelperLibrary.GetAIController` (`self.GetOwner`)))
  (bind _asaic_base_controller (cast `/Game/ShadowStep/Core/Blueprints/Enemy/Core/AI/AIC_BaseController` _returnvalue_2))
  (set `/Game/ShadowStep/Core/Blueprints/Enemy/Core/AI/AIC_BaseController.IsPaused` false _asaic_base_controller)
  (`Actor.SetActorTickEnabled` _returnvalue_2 true)
  (`BrainComponent.StartLogic` (`AIController.BrainComponent` _returnvalue_2))
  (`Actor.SetActorTickEnabled` _returnvalue true)
  (bind _ascharacter (cast `Character` _returnvalue))
  (`SkeletalMeshComponent.SetEnableAnimation` (`Character.Mesh` _ascharacter) true))

(fn `DeactivateArea`
  (bind _returnvalue (`self.GetOwner`))
  (bind _returnvalue_2 (`AIBlueprintHelperLibrary.GetAIController` (`self.GetOwner`)))
  (bind _asaic_base_controller (cast `/Game/ShadowStep/Core/Blueprints/Enemy/Core/AI/AIC_BaseController` _returnvalue_2))
  (set `/Game/ShadowStep/Core/Blueprints/Enemy/Core/AI/AIC_BaseController.IsPaused` true _asaic_base_controller)
  (`Actor.SetActorTickEnabled` _returnvalue_2 false)
  (`BrainComponent.StopLogic` (`AIController.BrainComponent` _returnvalue_2) "")
  (`Actor.SetActorTickEnabled` _returnvalue false)
  (bind _ascharacter (cast `Character` _returnvalue))
  (`SkeletalMeshComponent.SetEnableAnimation` (`Character.Mesh` _ascharacter) false))