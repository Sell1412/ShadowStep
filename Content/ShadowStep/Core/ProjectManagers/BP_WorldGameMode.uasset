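; World game mode for ShadowStep that manages checkpoints, player spawning and death resets.
; Checkpoints register themselves, the game-start one triggers spawning and possession of the player, and newly reached ones update the play area and save to a slot.
; On the player's death blackscreen, it teleports the character to the last checkpoint, broadcasts world reset, then fades the camera back in.
; It also creates and initializes the goal manager.
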(event `self.ReceiveBeginPlay`
  (`|ExecutionSequence`
    (:`then_0`
      (set `self.PlayerController` (`GameplayStatics.GetPlayerController` 0))
      (bind _asbp_player_charakter (cast `/Game/ShadowStep/Characters/Player/BP_PlayerCharakter` (`GameplayStatics.GetPlayerCharacter` 0)))
      (bind _output_get (set `self.Player Char` _asbp_player_charakter))
      (add `/Game/ShadowStep/Characters/Player/BP_PlayerCharakter.OnPlayerDeathBlackScreen` _output_get (delegate `OnPlayerDeathBlackScreen_Event`)))
    (:`then_1`
      (`self.SetUpGoalManager`))))

(event `OnPlayerDeathBlackScreen_Event`
  (`self.MovePlayerToCheckpoint`)
  (`self.Reset World`)
  (`KismetSystemLibrary.Delay` 1.0)
  (`PlayerCameraManager.StartCameraFade` :`self` (`GameplayStatics.GetPlayerCameraManager` 0) :`FromAlpha` 1.0 :`Duration` 0.6)
  (`self.OnWorldResetFinished`))

(event `OnSpawnPointSet`
  (`self.SpawnPlayer`)
  (`self.OnPlayerSpawned`)
  (set `self.PlayerIsSpawned` true))

(fn `LoadSaveCheckpointGame`
  (bind _returnvalue (`GameplayStatics.LoadGameFromSlot` (`self.Save Slot Name`)))
  (bind _asbp_save_game (cast `/Game/ShadowStep/Enviroment/Respawn/SaveGame/BP_SaveGame` _returnvalue))
  (`self.SetLoadedCheckpointData` _asbp_save_game))

(fn `MovePlayerToCheckpoint`
  (bind _returnvalue (`GameplayStatics.GetPlayerCharacter` 0))
  (bind _respawnpoint (`/Game/ShadowStep/Enviroment/Respawn/BP_Checkpoint.RespawnPoint` (`self.LastCheckpoint`)))
  (bind _returnvalue_2 (`SceneComponent.K2_GetComponentRotation` _respawnpoint))
  ; Set Charakter Location and Rotation
  (`self.K2_SetActorLocation` _returnvalue (`SceneComponent.K2_GetComponentLocation` _respawnpoint) false false)
  (`self.K2_SetActorRotation` _returnvalue _returnvalue_2 false)
  ; Set Look Direction
  (`Controller.SetControlRotation` (`Pawn.GetController` _returnvalue) _returnvalue_2))

(fn `RegisterCheckpoint`
  (params (checkpoint :type "/Game/ShadowStep/Enviroment/Respawn/BP_Checkpoint Object Reference"))
  (`KismetArrayLibrary.Array_AddUnique` (`self.AllCheckPoints`) checkpoint)
  (if (`/Game/ShadowStep/Enviroment/Respawn/BP_Checkpoint.IsGameStartPoint` checkpoint)
    (set `self.LastCheckpoint` checkpoint)
    (`self.OnSpawnPointSet`)
    (return)
    (else
      (return))))

(fn `Reset World`
  (`self.OnWorldReset`)
  (return))

(fn `SaveData`
  (params (SaveGameObj :type "/Game/ShadowStep/Enviroment/Respawn/SaveGame/BP_SaveGame Object Reference"))
  (set `/Game/ShadowStep/Enviroment/Respawn/SaveGame/BP_SaveGame.LastCheckpoint` (`self.LastCheckpoint`) SaveGameObj)
  (set `/Game/ShadowStep/Enviroment/Respawn/SaveGame/BP_SaveGame.OldCheckedPoints` (`self.OldCheckedPoints`) SaveGameObj))

(fn `SaveGame`
  (bind _returnvalue (`GameplayStatics.CreateSaveGameObject` "/Game/ShadowStep/Enviroment/Respawn/SaveGame/BP_SaveGame.BP_SaveGame_C"))
  (`self.SaveData` _returnvalue)
  (`GameplayStatics.SaveGameToSlot` _returnvalue (`self.Save Slot Name`)))

(fn `SetLoadedCheckpointData`
  (params (SaveGame :type "/Game/ShadowStep/Enviroment/Respawn/SaveGame/BP_SaveGame Object Reference"))
  (set `self.LastCheckpoint` (`/Game/ShadowStep/Enviroment/Respawn/SaveGame/BP_SaveGame.LastCheckpoint` SaveGame))
  (set `self.OldCheckedPoints` (`/Game/ShadowStep/Enviroment/Respawn/SaveGame/BP_SaveGame.OldCheckedPoints` SaveGame)))

(fn `SetNewCheckpoint`
  (params (NewCheckpoint :type "/Game/ShadowStep/Enviroment/Respawn/BP_Checkpoint Object Reference"))
  (returns (Sucessfull :type Boolean))
  (locals (newCheckpoint_l :type "/Game/ShadowStep/Enviroment/Respawn/BP_Checkpoint Object Reference"))
  (bind _output_get (set `local.newCheckpoint_l` NewCheckpoint))
  (if (== (`KismetArrayLibrary.Array_Find` (`self.OldCheckedPoints`) _output_get) -1)
    (`KismetArrayLibrary.Array_AddUnique` (`self.OldCheckedPoints`) (`local.newCheckpoint_l`))
    (bind _output_get_2 (set `self.LastCheckpoint` (`local.newCheckpoint_l`)))
    (set `self.CurrentPlayArea` (`Checkpoint.NewArea` _output_get_2))
    (`self.SaveGame`)
    (return true)
    (else
      (return false))))

(fn `SetUpGoalManager`
  (bind _returnvalue (`|GenericCreateObject` self "/Game/ShadowStep/Core/ProjectManagers/Managers/BP_GoalManager.BP_GoalManager_C"))
  (bind _output_get (set `self.GoalManager` _returnvalue))
  (`/Game/ShadowStep/Core/ProjectManagers/Managers/BP_GoalManager.Initialize` _output_get self))

(fn `SpawnPlayer`
  (bind _respawnlocation (`/Game/ShadowStep/Enviroment/Respawn/BP_Checkpoint.GetRespawnLocation` (`self.LastCheckpoint`)))
  (bind _returnvalue (`|SpawnActorFromClass` "/Game/ShadowStep/Characters/Player/BP_PlayerCharakter.BP_PlayerCharakter_C" _respawnlocation "AlwaysSpawn" "MultiplyWithRoot" (`GameplayStatics.GetPlayerController` 0) null))
  (`Controller.Possess` (`GameplayStatics.GetPlayerController` 0) _returnvalue)
  ;[0.5029 0.001518 0 0.502] RespawnSound
  (`GameplayAudioHelper.PlaySoundAttachedToActor` (struct :`TagName` "Audio.Sounds.Player.Respawn") _returnvalue))

(fn `UserConstructionScript`)