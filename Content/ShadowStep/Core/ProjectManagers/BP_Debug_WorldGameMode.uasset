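; BP_Debug_WorldGameMode is a game mode that records checkpoint progress and saves it to disk.
; SetNewCheckpoint ignores checkpoints already visited; a new one is added to the visited list, becomes LastCheckpoint, triggers a save and returns true.
; SaveGame creates a fresh BP_SaveGame, fills in the checkpoint and its respawn location through SaveData, and writes it to a single fixed slot.
; The visited list is not saved, and no loading happens here.
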(fn `SaveData`
  (params (self2 :type "/Game/Development/Tobias/Blueprints/Respawn/SaveGame/BP_SaveGame Object Reference"))
  (set `/Game/Development/Tobias/Blueprints/Respawn/SaveGame/BP_SaveGame.RespawnPos` (`/Game/Development/Tobias/Blueprints/Respawn/BP_Checkpoint.RespawnLocation` (`self.LastCheckpoint`)) self2)
  (set `/Game/Development/Tobias/Blueprints/Respawn/SaveGame/BP_SaveGame.LastCheckpoint` (`self.LastCheckpoint`) self2))

(fn `SaveGame`
  (bind _returnvalue (`GameplayStatics.CreateSaveGameObject` "/Game/Development/Tobias/Blueprints/Respawn/SaveGame/BP_SaveGame.BP_SaveGame_C"))
  (`self.SaveData` _returnvalue)
  (`GameplayStatics.SaveGameToSlot` _returnvalue "SaveGame"))

(fn `SetNewCheckpoint`
  (params (NewCheckpoint :type "/Game/Development/Tobias/Blueprints/Respawn/BP_Checkpoint Object Reference"))
  (returns (Sucessfull :type Boolean))
  (locals (newCheckpoint_l :type "/Game/Development/Tobias/Blueprints/Respawn/BP_Checkpoint Object Reference"))
  (bind _output_get (set `local.newCheckpoint_l` NewCheckpoint))
  (if (== (`KismetArrayLibrary.Array_Find` (`self.OldCheckedPoints`) _output_get) -1)
    (`KismetArrayLibrary.Array_AddUnique` (`self.OldCheckedPoints`) (`local.newCheckpoint_l`))
    (set `self.LastCheckpoint` (`local.newCheckpoint_l`))
    (`self.SaveGame`)
    (return true)
    (else
      (return false))))

(fn `UserConstructionScript`)