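; Game instance for ShadowStep that manages the pause and end-game UI widgets.
; OpenPauseMenu shows an existing pause widget, pausing the game and switching to UI-only input with cursor, or otherwise only creates it hidden.
; OpenEndGameMenu creates the end screen on a higher viewport layer, switches to UI input and plays its reveal animation without pausing.
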(fn `CreatePauseMenu`
  (bind _output_get (set `self.PlayerController` (`GameplayStatics.GetPlayerController` 0)))
  (bind _returnvalue (`|CreateWidget` "/Game/ShadowStep/UI/Menus/InGamePause/WBP_PauseMenu.WBP_PauseMenu_C" _output_get))
  (set `self.PauseMenu` _returnvalue)
  (`UserWidget.AddToViewport` (`self.PauseMenu`) 1)
  (`Widget.SetVisibility` (`self.PauseMenu`) "Hidden"))

(fn `OpenEndGameMenu`
  (bind _endgamemenu (`self.EndGameMenu`))
  (bind _output_get (set `self.PlayerController` (`GameplayStatics.GetPlayerController` 0)))
  (bind _returnvalue (`|CreateWidget` "/Game/ShadowStep/UI/Menus/EndGame/WBP_EndGameScreen.WBP_EndGameScreen_C" _output_get))
  (bind _output_get_2 (set `self.EndGameMenu` _returnvalue))
  (`UserWidget.AddToViewport` _output_get_2 2)
  (`WidgetBlueprintLibrary.SetInputMode_UIOnlyEx` (`self.PlayerController`) (`self.EndGameMenu`))
  (set `PlayerController.bShowMouseCursor` true (`self.PlayerController`))
  (`Widget.SetVisibility` _endgamemenu "Visible")
  (`UserWidget.PlayAnimation` (`self.EndGameMenu`) (`/Game/ShadowStep/UI/Menus/EndGame/WBP_EndGameScreen.ShowEndScreen` _endgamemenu) 0.0 1 "Forward" 1.0 false))

(fn `OpenPauseMenu`
  (`/Engine/EditorBlueprintResources/StandardMacros.IsValid` (`self.PauseMenu`)
    (:`Is Valid`
      (`self.ShowPauseMenu`))
    (:`Is Not Valid`
      (`self.CreatePauseMenu`))))

(fn `ShowPauseMenu`
  (`Widget.SetVisibility` (`self.PauseMenu`) "Visible")
  (`GameplayStatics.SetGamePaused` true)
  (`WidgetBlueprintLibrary.SetInputMode_UIOnlyEx` (`self.PlayerController`) (`self.PauseMenu`) "DoNotLock" true)
  (`/Game/ShadowStep/UI/Menus/InGamePause/WBP_PauseMenu.Focus` (`self.PauseMenu`))
  (set `PlayerController.bShowMouseCursor` true (`self.PlayerController`)))