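; Goal manager that tracks which goal target is the current objective in the play area.
; Initialize gathers every A_GoalTarget in the level and gives each a reference back to the manager for callbacks.
; It filters them by the Gamemode's current play area and selects the lowest step priority value as the current goal.
; Removing a goal triggers reselection, and a getter returns the current goal with its description or a placeholder.
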(fn `GetCurrentCoal`
  (returns (Object :type "/Game/Development/Tobias/Enviremoent/A_GoalTarget Object Reference") (Descpription :type Text))
  (bind _currentgoal (`self.CurrentGoal`))
  (`/Engine/EditorBlueprintResources/StandardMacros.IsValid` _currentgoal
    (:`Is Valid`
      (return _currentgoal (`/Game/Development/Tobias/Enviremoent/A_GoalTarget.Description` _currentgoal)))
    (:`Is Not Valid`
      (return null "-----"))))

(fn `Initialize`
  (params (Gamemode :type "/Game/ShadowStep/Core/ProjectManagers/BP_WorldGameMode Object Reference"))
  (bind _output_get (set `self.Gamemode` Gamemode))
  (bind _outactors (`GameplayStatics.GetAllActorsOfClass` _output_get "/Game/Development/Tobias/Enviremoent/A_GoalTarget.A_GoalTarget_C"))
  (bind _output_get_2 (set `self.AllGoalsInLevel` _outactors))
  ; Set The Manager inside the Goals for callback
  (for _array_element _output_get_2
    (set `/Game/Development/Tobias/Enviremoent/A_GoalTarget.GoalManager` self _array_element))
  (`self.UpdateNewArea`))

(fn `RemoveGoalFromList`
  (params (`Removing Target` :type "/Game/Development/Tobias/Enviremoent/A_GoalTarget Object Reference"))
  (bind _returnvalue (`KismetArrayLibrary.Array_Find` (`self.CurrentAreaGoals`) `Removing Target`))
  ; Find Checkpoint in Array
  (if (!= _returnvalue -1)
    (`KismetArrayLibrary.Array_Remove` (`self.CurrentAreaGoals`) _returnvalue)
    ; Update for New Goal
    (`self.UpdateNewGoal`)))

(fn `UpdateNewArea`
  (`KismetArrayLibrary.Array_Clear` (`self.CurrentAreaGoals`))
  (for _array_element (`self.AllGoalsInLevel`)
    (if (== (`/Game/Development/Tobias/Enviremoent/A_GoalTarget.GoalArea` _array_element) (`/Game/ShadowStep/Core/ProjectManagers/BP_WorldGameMode.CurrentPlayArea` (`self.Gamemode`)))
      (`KismetArrayLibrary.Array_Add` (`self.CurrentAreaGoals`) _array_element)))
  (`self.UpdateNewGoal`))

(fn `UpdateNewGoal`
  (locals (CurrentHighestPoint :type "/Game/Development/Tobias/Enviremoent/A_GoalTarget Object Reference") (TmpHighetsPrio :type "/Game/Development/Tobias/Enviremoent/A_GoalTarget Object Reference"))
  (bind _tmphighetsprio (`local.TmpHighetsPrio`))
  (for _array_element (`self.CurrentAreaGoals`)
    (`/Engine/EditorBlueprintResources/StandardMacros.IsValid` _tmphighetsprio
      (:`Is Valid`
        (if (< (`/Game/Development/Tobias/Enviremoent/A_GoalTarget.StepPriotirty` _array_element) (`/Game/Development/Tobias/Enviremoent/A_GoalTarget.StepPriotirty` _tmphighetsprio))
          (set `local.TmpHighetsPrio` _array_element :!label _label)))
      (:`Is Not Valid`
        ; Set the first element to Tmp
        (set `local.TmpHighetsPrio` _array_element)
        (goto _label))))
  (set `self.CurrentGoal` (`local.TmpHighetsPrio`)))