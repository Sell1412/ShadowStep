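; Player component that handles stealth executions of nearby enemies in ShadowStep.
; Add and remove functions maintain the nearby enemy list and fire matching notifications.
; On the kill input, the first listed enemy is snapped in front of the player, killed through its AI health component, and has its execute box disabled.
; The kill then reports a noise event at the player's location and plays a montage on the player mesh.
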(event `self.ReceiveBeginPlay`
  (bind _asbp_player_charakter (cast `/Game/ShadowStep/Characters/Player/BP_PlayerCharakter` (`self.GetOwner`)))
  (set `self.PlayerMesh` (`Character.Mesh` _asbp_player_charakter))
  (set `self.PlayerController` (`Pawn.GetController` _asbp_player_charakter)))

(event `EnhancedInput|/Game/ShadowStep/Input/Actions/IA_Kill`
  (params (ActionValue :type "Vector2D Structure") (ElapsedSeconds :type "Float (double-precision)") (TriggeredSeconds :type "Float (double-precision)") (InputAction :type "InputAction Object Reference" :default "/Game/ShadowStep/Input/Actions/IA_Kill.IA_Kill"))
  (bind _returnvalue (`self.GetOwner`))
  (bind _returnvalue_2 (`self.GetOwner`))
  (bind _returnvalue_3 (`Actor.GetActorForwardVector` _returnvalue_2))
  (:`Triggered`
    (if (> (`KismetArrayLibrary.Array_Length` (`self.NearbyEnemys`)) 0)
      (`SceneComponent.K2_SetWorldLocationAndRotation` (`Actor.RootComponent` (`|GetArrayItem` (`self.NearbyEnemys`))) (+ (`Actor.K2_GetActorLocation` _returnvalue_2) _returnvalue_3) (`KismetMathLibrary.Conv_VectorToRotator` _returnvalue_3) false false)
      ; Kill Enemy
      (`self.ExecuteEnemy` (`|GetArrayItem` (`self.NearbyEnemys`)))
      ; MakeSound
      (`AISense_Hearing.ReportNoiseEvent` (`Actor.K2_GetActorLocation` _returnvalue) 1.0 _returnvalue (`self.KillNoiceSoundRange`))
      (`|PlayMontage` (`self.PlayerMesh`) (`self.KillEnemyMontage`)))))

(fn `AddNearbyEnemy`
  (params (`New Enemy` :type "/Game/ShadowStep/Core/Blueprints/Enemy/Core/BP_EnemyBase Object Reference"))
  (`KismetArrayLibrary.Array_AddUnique` (`self.NearbyEnemys`) `New Enemy`)
  (`self.OnEnemyAdded` `New Enemy`))

(fn `ExecuteEnemy`
  (params (ToKilEnemy :type "/Game/ShadowStep/Core/Blueprints/Enemy/Core/BP_EnemyBase Object Reference"))
  (`/Engine/EditorBlueprintResources/StandardMacros.IsValid` ToKilEnemy
    (:`Is Valid`
      (`/Game/ShadowStep/Core/Blueprints/Enemy/Core/Component/AC_AIHealth.OnDeath` (`/Game/ShadowStep/Core/Blueprints/Enemy/Core/BP_EnemyBase.AC_AIHealth` ToKilEnemy))
      (`/Game/ShadowStep/Core/Blueprints/Enemy/Core/BP_EnemyBase.DisableExecuteBox` ToKilEnemy))))

(fn `RemoveNearbyEnemy`
  (params (`Removing Enemy` :type "/Game/ShadowStep/Core/Blueprints/Enemy/Core/BP_EnemyBase Object Reference"))
  (bind _returnvalue (`KismetArrayLibrary.Array_RemoveItem` (`self.NearbyEnemys`) `Removing Enemy`))
  (if _returnvalue
    (`self.OnEnemyRemove` `Removing Enemy`)))

(fn `Reset`
  (set `self.NearbyEnemys` (`|MakeArray` null :!type "/Game/ShadowStep/Core/Blueprints/Enemy/Core/BP_EnemyBase Object Reference"))
  (set `self.ToKillEnemy` null))