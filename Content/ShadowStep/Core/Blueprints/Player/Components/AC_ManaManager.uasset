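; Player mana component that regenerates mana in moonlight shadow and kills the player when a subtraction would drop it below zero.
; Unless flagged as in light, Tick traces from the capsule's base against the directional light's direction; a hit means shadow, adding mana and enabling a Niagara indicator.
; Mana changes fire update, gain or loss notifications, while regeneration plays an attached sound until stopped.
; It also offers ability cost checks and a reset.
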(event `self.ReceiveBeginPlay`
  (set `self.CurrentManaPoints` (`self.MaxManaPoints`))
  (`self.OnManaUpdated`)
  (bind _returnvalue (`GameplayStatics.GetActorOfClass` "/Script/Engine.DirectionalLight"))
  (set `self.MoonLightDirection` (`Actor.GetActorForwardVector` _returnvalue))
  (set `self.PlayerHealth` (`Actor.GetComponentByClass` (`self.GetOwner`) "/Game/ShadowStep/Core/Blueprints/Player/Components/AC_PlayerHealth.AC_PlayerHealth_C"))
  (set `self.PlayerHalfHeight` (`CapsuleComponent.CapsuleHalfHeight` (`Actor.GetComponentByClass` (`self.GetOwner`) "/Script/Engine.CapsuleComponent")))
  (set `self.ShadowIndicator` (`Actor.GetComponentByClass` (`self.GetOwner`) "/Script/Niagara.NiagaraComponent")))

(event `self.ReceiveTick`
  (params (DeltaSeconds :type "Float (single-precision)"))
  (if (not (`self.IsInLight`))
    (bind _isinshadow (`self.IsInShadow`))
    ; In shadow logic
    (if _isinshadow
      (`self.AddMana` (* DeltaSeconds (`self.ShadowHeal`)))
      ;; Is Shadow Niagara active
      (if (not (`self.IsShadowNiagraActive`))
        (`self.SetActive` (`self.ShadowIndicator`) true false)
        (set `self.IsShadowNiagraActive` true))
      (else
        ; Is Shadow Niagara deactivaded
        (if (`self.IsShadowNiagraActive`)
          (`self.SetActive` (`self.ShadowIndicator`) false false)
          (set `self.IsShadowNiagraActive` false)
          (`self.StopRegenAudio`))))))

(fn `AddMana`
  (params (ManaAmount :type "Float (double-precision)"))
  (bind _returnvalue (+ ManaAmount (`self.CurrentManaPoints`)))
  ; Check if mana points are at max
  (if (< _returnvalue (`self.MaxManaPoints`))
    ; Only update mana when mana points changed
    (set `self.CurrentManaPoints` _returnvalue)
    (`self.OnManaUpdated`)
    (`self.OnManaGain`)
    (`/Engine/EditorBlueprintResources/StandardMacros.IsValid` (`self.ManaRegenAudio`)
      (:`Is Not Valid`
        (bind _returnvalue_2 (`GameplayAudioHelper.PlaySoundAttachedToActor` (struct :`TagName` "Audio.Sounds.Player.Regen") (`GameplayStatics.GetPlayerCharacter` 0)))
        (set `self.ManaRegenAudio` _returnvalue_2)))
    (else
      ; Hold mana at max
      (set `self.CurrentManaPoints` (`self.MaxManaPoints`))
      (`self.StopRegenAudio`)))
  (return))

(fn `IsInShadow`
  (returns (IsInShadow :type Boolean))
  (bind (_returnvalue_x _returnvalue_y _returnvalue_z) (`KismetMathLibrary.BreakVector` (`Actor.K2_GetActorLocation` (`self.GetOwner`))))
  (bind _returnvalue (`KismetMathLibrary.MakeVector` _returnvalue_x _returnvalue_y (- _returnvalue_z (`self.PlayerHalfHeight`))))
  (bind (_outhit _returnvalue_2) (`KismetSystemLibrary.LineTraceSingle` :`Start` _returnvalue :`End` (+ _returnvalue (* (`KismetMathLibrary.NegateVector` (`self.MoonLightDirection`)) (`self.MoonLightShadowCheckLength`))) :`TraceChannel` "TraceTypeQuery1" :`DrawTime` 2.0))
  (if _returnvalue_2
    (return true)
    (else
      (return false))))

(fn `RequestAbilityUseage`
  (params (ManaCost :type "Float (double-precision)"))
  (returns (AbilityUsable :type Boolean))
  (if (< ManaCost (`self.CurrentManaPoints`))
    (return true)
    (else
      (return false))))

(fn `Reset`
  (set `self.IsInLight` false)
  (set `self.CurrentManaPoints` (`self.MaxManaPoints`))
  (`self.OnManaUpdated`))

(fn `SetIsInLight`
  (params (IsInLight :type Boolean))
  (set `self.IsInLight` IsInLight))

(fn `StopRegenAudio`
  (bind _manaregenaudio (`self.ManaRegenAudio`))
  (`/Engine/EditorBlueprintResources/StandardMacros.IsValid` _manaregenaudio
    (:`Is Valid`
      (`AudioComponent.Stop` _manaregenaudio)
      (set `self.ManaRegenAudio` null))))

(fn `SubtractMana`
  (params (ManaSubtractionMultiplier :type "Float (double-precision)"))
  (bind _returnvalue (- (`self.CurrentManaPoints`) ManaSubtractionMultiplier))
  (if (>= _returnvalue 0.0)
    (set `self.CurrentManaPoints` _returnvalue)
    (`self.OnManaUpdated`)
    (`self.OnManaLose`)
    (return)
    (else
      (`/Game/ShadowStep/Core/Blueprints/Player/Components/AC_PlayerHealth.KillPlayer` (`self.PlayerHealth`))
      (`self.OnManaUpdated`)
      (`self.OnManaLose`))))