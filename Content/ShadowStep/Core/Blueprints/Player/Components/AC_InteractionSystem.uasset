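; Player interaction component that finds interactables in the camera's view and drives press-and-hold interaction.
; Each tick it sphere-traces from the camera, showing or hiding prompts on BPI_Interactable actors through interface messages.
; IA_Interact locks move and look input while held and sends interaction start and end messages.
; Losing the trace hit or player death also ends an active interaction, and Reset clears the state.
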(event `self.ReceiveBeginPlay`
  (set `self.CameraManager` (`GameplayStatics.GetPlayerCameraManager` 0))
  (bind _output_get (set `self.PlayerHealth` (`Actor.GetComponentByClass` (`self.GetOwner`) "/Game/ShadowStep/Core/Blueprints/Player/Components/AC_PlayerHealth.AC_PlayerHealth_C")))
  (add `/Game/ShadowStep/Core/Blueprints/Player/Components/AC_PlayerHealth.OnPlayerDeath` _output_get (`|CreateDelegate` :!event `PlayerDied`))
  (set `self.PlayerController` (`GameplayStatics.GetPlayerController` 0))
  (bind _asbp_player_charakter (cast `/Game/ShadowStep/Characters/Player/BP_PlayerCharakter` (`self.GetOwner`)))
  (set `self.PlayerCharacter` _asbp_player_charakter))

(event `self.ReceiveTick`
  (params (DeltaSeconds :type "Float (single-precision)"))
  (bind _cameramanager (`self.CameraManager`))
  (bind _interactableactor (`self.InteractableActor`))
  (bind _returnvalue (`PlayerCameraManager.GetCameraLocation` _cameramanager))
  ; Scan for Interatables
  (bind (_outhit _returnvalue_2) (`KismetSystemLibrary.SphereTraceSingle` _returnvalue (+ _returnvalue (* (`KismetMathLibrary.GetForwardVector` (`PlayerCameraManager.GetCameraRotation` _cameramanager)) (`self.InteractionLength`))) (`self.SphereRadius`) "TraceTypeQuery3"))
  (if _returnvalue_2
    (bind (_bblockinghit _binitialoverlap _time _distance _location _impactpoint _normal _impactnormal _physmat _hitactor) (`GameplayStatics.BreakHitResult` _outhit))
    ; Does object implement interface
    (if (`KismetSystemLibrary.DoesImplementInterface` _hitactor "/Game/Development/Justin/Interface/BPI_Interactable.BPI_Interactable_C")
      ; Check for not equal interactable
      (if (!= (`self.InteractableActor`) _hitactor)
        ; Hide interaction from old interactable
        (message `/Game/Development/Justin/Interface/BPI_Interactable.HideInteraction` (`self.InteractableActor`))
        ; Show interaction by new one
        (bind _output_get (set `self.InteractableActor` _hitactor))
        (message `/Game/Development/Justin/Interface/BPI_Interactable.ShowInteraction` _output_get)))
    (else
      ; Hide interaction
      (`/Engine/EditorBlueprintResources/StandardMacros.IsValid` _interactableactor
        (:`Is Valid`
          (message `/Game/Development/Justin/Interface/BPI_Interactable.HideInteraction` _interactableactor)
          ; Set interatable object in valid
          (if (`self.PressedInteraction`)
            (message `/Game/Development/Justin/Interface/BPI_Interactable.InteractEnded` (`self.InteractableActor`)))
          (set `self.InteractableActor` null))))))

(event `EnhancedInput|/Game/ShadowStep/Input/Actions/IA_Interact`
  (params (ActionValue :type "Vector2D Structure") (ElapsedSeconds :type "Float (double-precision)") (TriggeredSeconds :type "Float (double-precision)") (InputAction :type "InputAction Object Reference" :default "/Game/ShadowStep/Input/Actions/IA_Interact.IA_Interact"))
  (bind _playercontroller (`self.PlayerController`))
  (bind _playercontroller_2 (`self.PlayerController`))
  (:`Started`
    ; Lock Move and Look Input
    (`Controller.SetIgnoreMoveInput` _playercontroller_2 true)
    (`Controller.SetIgnoreLookInput` _playercontroller_2 true)
    ; Check if interactable actor exists
    (`/Engine/EditorBlueprintResources/StandardMacros.IsValid` (`self.InteractableActor`)
      (:`Is Valid`
        ; Start interaction
        (set `self.PressedInteraction` true)
        (message `/Game/Development/Justin/Interface/BPI_Interactable.InteractStarted` (`self.InteractableActor`)))))
  (:`Canceled`
    ; Unlock Move and Look Input
    (`Controller.SetIgnoreMoveInput` _playercontroller false :!label _label)
    (`Controller.SetIgnoreLookInput` _playercontroller false)
    ; Check if interaction was started
    (if (`self.PressedInteraction`) :!label _label_2
      ; End interaction
      (set `self.PressedInteraction` false)
      (message `/Game/Development/Justin/Interface/BPI_Interactable.InteractEnded` (`self.InteractableActor`))))
  (:`Completed`
    (goto _label)))

(event `PlayerDied`
  (goto _label_2))

(fn `Reset`
  (set `self.InteractableActor` null)
  (set `self.PressedInteraction` false))