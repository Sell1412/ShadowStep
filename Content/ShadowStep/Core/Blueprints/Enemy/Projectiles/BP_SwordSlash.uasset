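; BP_SwordSlash is an enemy sword slash projectile that kills the player on contact.
; When its SlashHitBox overlaps the player character, it calls KillPlayer on the player's health component and plays an attached hit sound by tag.
; It destroys itself shortly after a hit, or when the lifetime timer set on BeginPlay expires.
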(event `self.ReceiveBeginPlay`
  (`KismetSystemLibrary.K2_SetTimerDelegate` (delegate `DestroySelf`) 2.0))

(event `DestroySelf`
  (`self.K2_DestroyActor`))

(event `self.SlashHitBox.OnComponentBeginOverlap`
  (params (OverlappedComponent :type "PrimitiveComponent Object Reference") (OtherActor :type "Actor Object Reference") (OtherComp :type "PrimitiveComponent Object Reference") (OtherBodyIndex :type Integer) (bFromSweep :type Boolean) (SweepResult :type "HitResult Structure (by ref)"))
  (if (== OtherActor (`GameplayStatics.GetPlayerCharacter` 0))
    ; If Player is Hit
    (bind _asbp_player_charakter (cast `/Game/ShadowStep/Characters/Player/BP_PlayerCharakter` OtherActor))
    (`/Game/ShadowStep/Core/Blueprints/Player/Components/AC_PlayerHealth.KillPlayer` (`/Game/ShadowStep/Characters/Player/BP_PlayerCharakter.AC_PlayerHealth` _asbp_player_charakter))
    (`GameplayAudioHelper.PlaySoundAttachedToActor` (struct :`TagName` "Audio.Sounds.Enemy.SlashHit") self)
    (`KismetSystemLibrary.Delay` 0.5)
    (`self.DestroySelf`)))

(fn `UserConstructionScript`)