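; AC_AIComponent is an actor component that provides AI state helpers for enemies.
; It sets a sword enemy's walk speed from configurable patrol, search and chase speeds based on the given mode.
; It also writes a starting EnemyState enum into the owner's AI controller blackboard and can reset its NearbyEnemys array.
; Begin Play and Tick are empty.
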(event `self.ReceiveBeginPlay`)

(event `self.ReceiveTick`
  (params (DeltaSeconds :type "Float (single-precision)")))

(fn `Reset`
  (set `self.Nearby Enemys` (`|MakeArray` null :!type "/Game/ShadowStep/Core/Blueprints/Enemy/Core/BP_EnemyBase Object Reference")))

(fn `SetMovementSpeedOnState`
  (params (Pawn :type "Pawn Object Reference") (Mode :type "/Game/ShadowStep/Core/Blueprints/Enemy/Core/Enum/E_EnemyState Enum" :default "NewEnumerator0"))
  (bind _asbp_sword_enemy (cast `/Game/ShadowStep/Characters/Enemy/BP_SwordEnemy` Pawn)
    (:`then`
      (set `CharacterMovementComponent.MaxWalkSpeed` (select `/Game/ShadowStep/Core/Blueprints/Enemy/Core/Enum/E_EnemyState` Mode :`NewEnumerator0` (`self.PatrolMovementSpeed`) :`NewEnumerator1` (`self.SearchMovementSpeed`) :`NewEnumerator2` (`self.ChaseMovementSpeed`)) (`Character.CharacterMovement` _asbp_sword_enemy))
      (return))
    (:`CastFailed`
      (return))))

(fn `SetStartState`
  (params (EnumValue :type Byte))
  (`BlackboardComponent.SetValueAsEnum` (`AIBlueprintHelperLibrary.GetBlackboard` (`AIBlueprintHelperLibrary.GetAIController` (`self.GetOwner`))) "EnemyState" EnumValue))