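; BP_GoalEnemy is an enemy character whose death ends the game.
; When its AC_AIHealth component fires OnEnemyDeath, it disables move and look input on the first player controller.
; It then casts the game instance to BP_WorldGameInstance and opens the end-game menu.
; BeginPlay, overlap and Tick are disabled stubs, so the death handler is its only active event logic.
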(event `self.AC_AIHealth.OnEnemyDeath`
  (bind _returnvalue (`GameplayStatics.GetPlayerController` 0))
  (`Controller.SetIgnoreMoveInput` _returnvalue true)
  (`Controller.SetIgnoreLookInput` _returnvalue true)
  (bind _asbp_world_game_instance (cast `/Game/ShadowStep/Core/ProjectManagers/BP_WorldGameInstance` (`GameplayStatics.GetGameInstance`)))
  (`/Game/ShadowStep/Core/ProjectManagers/BP_WorldGameInstance.OpenEndGameMenu` _asbp_world_game_instance))

(fn `UserConstructionScript`
  (`parent.UserConstructionScript`))