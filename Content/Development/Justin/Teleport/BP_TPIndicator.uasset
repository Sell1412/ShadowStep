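; BP_TPIndicator is a teleport indicator actor with a sphere that can be moved, hidden and tested for being in shadow.
; It maintains a list of lights in range through add and remove functions that print debug messages.
; IsInShadow line-traces to each light on the Visibility channel, stopping at the first unblocked one.
; SetVisibility passes its input straight through as the hidden flag, so true hides the indicator.
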(fn `AddLightInRange`
  (params (BaseLight :type "/Game/Development/Justin/Teleport/BP_LightBase Object Reference"))
  (`KismetArrayLibrary.Array_Add` (`self.LightsInRange`) BaseLight)
  (`KismetSystemLibrary.PrintString` "Added light" true true (struct :`R` 1.0 :`G` 0.021726 :`A` 1.0)))

(fn `IsInShadow`
  (returns (InShadow :type Boolean))
  (locals (ObjectHitted :type Boolean :default true))
  (for _array_element (`self.LightsInRange`)
    (bind (_outhit _returnvalue) (`KismetSystemLibrary.LineTraceSingle` :`Start` (`SceneComponent.K2_GetComponentLocation` (`self.DefaultSceneRoot`)) :`End` (`SceneComponent.K2_GetComponentLocation` (`/Game/Development/Justin/Teleport/BP_LightBase.DefaultSceneRoot` _array_element)) :`TraceChannel` "TraceTypeQuery1" :`TraceColor` (struct :`R` 1.0 :`B` 1.0 :`A` 1.0) :`DrawTime` 2.0))
    (bind _output_get (set `local.ObjectHitted` _returnvalue))
    (if (not _output_get)
      (break)))
  (return (`local.ObjectHitted`)))

(fn `RemoveLight`
  (params (ToRemoveLight :type "/Game/Development/Justin/Teleport/BP_LightBase Object Reference"))
  (bind _returnvalue (`KismetArrayLibrary.Array_RemoveItem` (`self.LightsInRange`) ToRemoveLight))
  (if _returnvalue
    (`KismetSystemLibrary.PrintString` "Sucessfully Removed Light" true true (struct :`R` 1.0 :`G` 0.058083 :`A` 1.0))
    (else
      (`KismetSystemLibrary.PrintString` "Did not Find light" true true (struct :`R` 1.0 :`G` 0.104536 :`A` 1.0)))))

(fn `SetVisibility`
  (params (Visibility :type Boolean))
  (`SceneComponent.SetHiddenInGame` (`self.Sphere`) Visibility true)
  (`SceneComponent.SetHiddenInGame` (`self.DefaultSceneRoot`) Visibility true))

(fn `SetWorldPostion`
  (params (NewPostion :type "Transform Structure"))
  (`SceneComponent.K2_SetWorldTransform` (`self.DefaultSceneRoot`) NewPostion false false))

(fn `UserConstructionScript`)