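; Actor component that gives its owner an aimed teleport into shadowed spots, limited by range and cooldown.
; While the input is held, Tick traces from the camera, snapping wall hits onto nearby ledges.
; Targets must pass a trace toward the DirectionalLight and the spawned indicator's shadow check, then get offset by surface slope.
; On release or cancel, a grounded owner moves to the valid point; a spawned range indicator toggles with aiming.
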(event `self.ReceiveBeginPlay`
  (bind _returnvalue (`self.GetOwner`))
  (set `self.CameraComponent` (`Actor.GetComponentByClass` (`self.GetOwner`) "/Script/Engine.CameraComponent"))
  (bind _returnvalue_2 (`GameplayStatics.GetActorOfClass` "/Script/Engine.DirectionalLight"))
  (bind _output_get (set `self.DirectionLight` _returnvalue_2))
  (`/Engine/EditorBlueprintResources/StandardMacros.IsValid` _output_get
    (:`Is Valid`
      (bind _returnvalue_3 (`|SpawnActorFromClass` "/Game/Development/Justin/Teleport/BP_RangeIndicator.BP_RangeIndicator_C" (`Actor.GetTransform` _returnvalue) "Undefined" "MultiplyWithRoot" _returnvalue null))
      (bind _output_get_2 (set `self.RangeInicatorRef` _returnvalue_3))
      (`Actor.K2_AttachToActor` _output_get_2 (`GameplayStatics.GetPlayerCharacter` 0) "None" "KeepWorld" "KeepWorld" "KeepWorld" true)
      (`SceneComponent.SetVisibility` (`/Game/Development/Justin/Teleport/BP_RangeIndicator.DefaultSceneRoot` (`self.RangeInicatorRef`)) false true)
      (`/Game/Development/Justin/Teleport/BP_RangeIndicator.SetRadius` (`self.RangeInicatorRef`) (`self.TPRange`))
      (set `self.CharacterMovementComponent` (`Actor.GetComponentByClass` (`self.GetOwner`) "/Script/Engine.CharacterMovementComponent"))
      (bind _output_get_3 (set `self.TPLocation` (0.0 0.0 0.0)))
      (bind _returnvalue_4 (`|SpawnActorFromClass` "/Game/Development/Justin/Teleport/BP_TPIndicator.BP_TPIndicator_C" (`KismetMathLibrary.Conv_VectorToTransform` _output_get_3) "Undefined" "MultiplyWithRoot" null null))
      (bind _output_get_4 (set `self.TPIndicator` _returnvalue_4))
      (`/Game/Development/Justin/Teleport/BP_TPIndicator.SetVisibility` _output_get_4 false))
    (:`Is Not Valid`
      (`KismetSystemLibrary.PrintString` "No Direction Light founded" true true (struct :`R` 1.0 :`A` 1.0) 500.0))))

(event `self.ReceiveTick`
  (params (DeltaSeconds :type "Float (single-precision)"))
  (bind _cameracomponent (`self.CameraComponent`))
  (bind (_bblockinghit _binitialoverlap _time _distance _location _impactpoint _normal) (`GameplayStatics.BreakHitResult` (`self.ToCheckHitResult`)))
  (bind _returnvalue (`SceneComponent.K2_GetComponentLocation` _cameracomponent))
  (bind (_bblockinghit_2 _binitialoverlap_2 _time_2 _distance_2 _location_2 _impactpoint_2 _normal_2) (`GameplayStatics.BreakHitResult` (`self.ToCheckHitResult`)))
  (bind _returnvalue_2 (+ _location _normal))
  (bind _returnvalue_3 (+ (+ (`.ImpactPoint` (`GameplayStatics.BreakHitResult` (`self.ToCheckHitResult`))) (* (`KismetMathLibrary.Normal` (`KismetMathLibrary.MakeVector` (.x (`SceneComponent.GetForwardVector` (`self.CameraComponent`))) (.y (`SceneComponent.GetForwardVector` (`self.CameraComponent`))))) 50.0)) (0.0 0.0 250.0)))
  (if (`self.ShowTPIndicator`)
    (bind (_outhit _returnvalue_4) (`KismetSystemLibrary.LineTraceSingle` :`Start` _returnvalue :`End` (+ _returnvalue (* (`SceneComponent.GetForwardVector` _cameracomponent) (`self.TPRange`))) :`TraceChannel` "TraceTypeQuery1" :`DrawTime` 2.0))
    (bind _output_get (set `self.ToCheckHitResult` _outhit))
    (if _returnvalue_4
      (bind _output_get_2 (set `self.Normal` (`.Normal` (`GameplayStatics.BreakHitResult` _output_get))))
      ; Hitpoint at a wall?
      (if (`KismetMathLibrary.InRange_FloatFloat` (`KismetMathLibrary.Dot_VectorVector` _output_get_2 (`KismetMathLibrary.Vector_Up`)) -0.17 0.17)
        ; Is TP Point not under a wall
        (bind (_outhit_2 _returnvalue_5) (`KismetSystemLibrary.LineTraceSingle` :`Start` _returnvalue_2 :`End` (+ _returnvalue_2 (0.0 0.0 250.0)) :`TraceChannel` "TraceTypeQuery1" :`TraceColor` (struct :`G` 1.0 :`B` 0.958032 :`A` 1.0) :`DrawTime` 20.0))
        (if (not _returnvalue_5)
          (bind (_outhit_3 _returnvalue_6) (`KismetSystemLibrary.LineTraceSingle` :`Start` _returnvalue_3 :`End` (+ _returnvalue_3 (0.0 0.0 -400.0)) :`TraceChannel` "TraceTypeQuery1" :`TraceColor` (struct :`R` 0.395589 :`B` 1.0 :`A` 1.0) :`DrawTime` 20.0))
          (if _returnvalue_6
            (if (<= (.z (- (`.Location` (`GameplayStatics.BreakHitResult` _outhit_3)) (`.Location` (`GameplayStatics.BreakHitResult` (`self.ToCheckHitResult`))))) 50.0)
              (set `self.ToCheckHitResult` _outhit_3)))))
      (bind _output_get_3 (set `self.TPLocation` _location_2))
      (bind _output_get_4 (set `self.Normal` _normal_2))
      (bind (_outhit_4 _returnvalue_7) (`KismetSystemLibrary.LineTraceSingle` (+ _output_get_3 _output_get_4) (+ _location_2 (* (`KismetMathLibrary.NegateVector` (`SceneComponent.GetForwardVector` (`Light.LightComponent` (`self.DirectionLight`)))) (`self.ShadowCheckLength`))) "TraceTypeQuery1"))
      (if _returnvalue_7
        (`/Game/Development/Justin/Teleport/BP_TPIndicator.SetWorldPostion` (`self.TPIndicator`) (`KismetMathLibrary.MakeTransform` (+ (* (`self.Normal`) (`self.TPIconPostionOffset`)) (`self.TPLocation`)) (`KismetMathLibrary.MakeRotFromZ` (`self.Normal`))))
        (bind _inshadow (`/Game/Development/Justin/Teleport/BP_TPIndicator.IsInShadow` (`self.TPIndicator`)))
        (if _inshadow
          (set `self.IsLocationValid` true)
          (if (<= (`self.MaxWallSlope`) (`KismetMathLibrary.Dot_VectorVector` (`self.Normal`) (`KismetMathLibrary.Vector_Up`)))
            (set `self.ModifyedTPLocation` (+ (* (`self.Normal`) (`self.TPGroundPostionLength`)) (`self.TPLocation`)))
            (else
              (set `self.ModifyedTPLocation` (+ (* (`self.Normal`) (`self.TPWallPostionOffset`)) (`self.TPLocation`)))))
          (else
            (`self.SetLocationNotValid`)))
        (else
          (`self.SetLocationNotValid`)))
      (else
        (`self.SetLocationNotValid`)))))

(event `EnhancedInput|/Game/Development/Tobias/ThirdPerson/Input/Actions/IA_Teleport`
  (params (ActionValue :type Boolean) (ElapsedSeconds :type "Float (double-precision)") (TriggeredSeconds :type "Float (double-precision)") (InputAction :type "InputAction Object Reference" :default "/Game/Development/Tobias/ThirdPerson/Input/Actions/IA_Teleport.IA_Teleport"))
  (bind _charactermovementcomponent (`self.CharacterMovementComponent`))
  (:`Started`
    (set `self.ShowTPIndicator` true)
    (`SceneComponent.ToggleVisibility` (`/Game/Development/Justin/Teleport/BP_RangeIndicator.DefaultSceneRoot` (`self.RangeInicatorRef`)) true))
  (:`Canceled`
    ; Teleport to Validpoint
    (`SceneComponent.ToggleVisibility` (`/Game/Development/Justin/Teleport/BP_RangeIndicator.DefaultSceneRoot` (`self.RangeInicatorRef`)) true :!label _label)
    (set `self.ShowTPIndicator` false)
    (if (`self.CanTeleport`)
      (if (`self.IsLocationValid`)
        (if (`NavMovementInterface.IsMovingOnGround` _charactermovementcomponent)
          (`MovementComponent.StopMovementImmediately` _charactermovementcomponent)
          (`Actor.K2_SetActorLocation` (`self.GetOwner`) (`self.ModifyedTPLocation`) false true)
          (set `self.CanTeleport` false)
          (`/Game/Development/Justin/Teleport/BP_TPIndicator.SetVisibility` (`self.TPIndicator`) false)
          (`KismetSystemLibrary.Delay` (`self.TPRefresh`))
          (set `self.CanTeleport` true))
        (else
          (`/Game/Development/Justin/Teleport/BP_TPIndicator.SetVisibility` (`self.TPIndicator`) false)))))
  (:`Completed`
    (goto _label)))

(fn `CallculateAimLocation`
  (returns (OutHit :type "HitResult Structure"))
  (bind _cameracomponent (`self.CameraComponent`))
  (bind _returnvalue (`SceneComponent.K2_GetComponentLocation` _cameracomponent))
  ; Hit where to Teleport
  (bind (_outhit _returnvalue_2) (`KismetSystemLibrary.LineTraceSingle` :`Start` _returnvalue :`End` (+ _returnvalue (* (`SceneComponent.GetForwardVector` _cameracomponent) (`self.TPRange`))) :`TraceChannel` "TraceTypeQuery1" :`DrawTime` 2.0))
  (set `self.ToCheckHitResult` _outhit)
  (if _returnvalue_2
    (return (`self.ToCheckHitResult`))
    (else
      (set `self.TPLocation` (0.0 0.0 0.0))
      (set `self.Normal` (0.0 0.0 0.0))
      (set `self.IsLocationValid` false)
      (`/Game/Development/Justin/Teleport/BP_TPIndicator.SetVisibility` (`self.TPIndicator`) false))))

(fn `SetLocationNotValid`
  (set `self.TPLocation` (0.0 0.0 0.0))
  (set `self.Normal` (0.0 0.0 0.0))
  (set `self.IsLocationValid` false)
  (`/Game/Development/Justin/Teleport/BP_TPIndicator.SetVisibility` (`self.TPIndicator`) false)
  (set `self.ToCheckHitResult` (struct)))