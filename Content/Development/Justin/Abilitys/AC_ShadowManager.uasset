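; AC_ShadowManager is a component that manages the player's three shadow abilities: teleport, light and shadow stone.
; BeginPlay constructs and initialises each ability object, defaults to teleport, creates a mana bar widget and caches the player character.
; Input actions switch abilities via deactivate/activate or start and release the current one, broadcasting changes and use.
; Tick forwards to the current ability only when the player's GetIsAlive returns false.
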(event `self.ReceiveBeginPlay`
  (bind _returnvalue (`|GenericCreateObject` "/Game/Development/Justin/Abilitys/Teleport/O_ShadowAbility_TP.O_ShadowAbility_TP_C"))
  (bind _output_get (set `self.ShadowTPAbility` _returnvalue))
  (`BaseAbility.InitialiseAbility` _output_get self)
  (set `self.CurrentAbility` (`self.ShadowTPAbility`))
  (bind _returnvalue_2 (`|GenericCreateObject` "/Game/Development/Justin/Abilitys/Light/O_ShadowAbility_Light.O_ShadowAbility_Light_C"))
  (bind _output_get_2 (set `self.ShadowLightAbility` _returnvalue_2))
  (`BaseAbility.InitialiseAbility` _output_get_2 self)
  (bind _returnvalue_3 (`|GenericCreateObject` "/Game/Development/Justin/Abilitys/ShadowStone/O_ShadowAbility_ShadowStone.O_ShadowAbility_ShadowStone_C"))
  (bind _output_get_3 (set `self.ShadowStoneAbility` _returnvalue_3))
  (`BaseAbility.InitialiseAbility` _output_get_3 self)
  (bind _returnvalue_4 (`|GenericCreateObject` "/Game/ShadowStep/UI/Player/ManaBar/WBP_ManaBar.WBP_ManaBar_C"))
  (set `self.ManaBar` _returnvalue_4)
  (bind _asbp_player_charakter (cast `/Game/ShadowStep/Characters/Player/BP_PlayerCharakter` (`GameplayStatics.GetPlayerCharacter` 0)))
  (set `self.As BP Player Charakter` _asbp_player_charakter)
  (`self.OnSetupFinished`))

(event `self.ReceiveTick`
  (params (DeltaSeconds :type "Float (single-precision)"))
  (bind _isplayerdead (`/Game/ShadowStep/Characters/Player/BP_PlayerCharakter.GetIsAlive` (`self.As BP Player Charakter`)))
  (if (not _isplayerdead)
    (`BaseAbility.AbilityTick` (`self.CurrentAbility`))))

(event `EnhancedInput|/Game/ShadowStep/Input/Actions/Ability/IA_UseAbility`
  (params (ActionValue :type Boolean) (ElapsedSeconds :type "Float (double-precision)") (TriggeredSeconds :type "Float (double-precision)") (InputAction :type "InputAction Object Reference" :default "/Game/ShadowStep/Input/Actions/Ability/IA_UseAbility.IA_UseAbility"))
  (bind _currentability (`self.CurrentAbility`))
  (:`Started`
    (`BaseAbility.StartInteraction` _currentability))
  (:`Canceled`
    (`BaseAbility.ReleaseInteraction` _currentability :!label _label)
    (`self.OnAbilityUsed` (`self.CurrentAbility`)))
  (:`Completed`
    (goto _label)))

(event `EnhancedInput|/Game/ShadowStep/Input/Actions/Ability/IA_ShadowTeleportion`
  (params (ActionValue :type Boolean) (ElapsedSeconds :type "Float (double-precision)") (TriggeredSeconds :type "Float (double-precision)") (InputAction :type "InputAction Object Reference" :default "/Game/ShadowStep/Input/Actions/Ability/IA_ShadowTeleportion.IA_ShadowTeleportion"))
  (:`Triggered`
    (`self.ChangeAbility` (`self.ShadowTPAbility`))))

(event `EnhancedInput|/Game/ShadowStep/Input/Actions/Ability/IA_ShadowLight`
  (params (ActionValue :type Boolean) (ElapsedSeconds :type "Float (double-precision)") (TriggeredSeconds :type "Float (double-precision)") (InputAction :type "InputAction Object Reference" :default "/Game/ShadowStep/Input/Actions/Ability/IA_ShadowLight.IA_ShadowLight"))
  (:`Triggered`
    (`self.ChangeAbility` (`self.ShadowLightAbility`))))

(event `EnhancedInput|/Game/ShadowStep/Input/Actions/Ability/IA_ShadowStone`
  (params (ActionValue :type Boolean) (ElapsedSeconds :type "Float (double-precision)") (TriggeredSeconds :type "Float (double-precision)") (InputAction :type "InputAction Object Reference" :default "/Game/ShadowStep/Input/Actions/Ability/IA_ShadowStone.IA_ShadowStone"))
  (:`Triggered`
    (`self.ChangeAbility` (`self.ShadowStoneAbility`))))

(fn `ChangeAbility`
  (params (NewAbility :type "BaseAbility Object Reference"))
  (bind _currentability (`self.CurrentAbility`))
  (`BaseAbility.DeactivateAbility` (`self.CurrentAbility`))
  (set `self.CurrentAbility` NewAbility)
  (`BaseAbility.ActivateAbility` _currentability)
  (`self.OnAbilityChange` (`BaseAbility.shadowAbilityType` _currentability)))

(fn `GetCurrentAbility`
  (returns (AbilityName :type "EShadowAbilityType Enum"))
  (return (`BaseAbility.shadowAbilityType` (`self.CurrentAbility`))))

(fn `Reset`
  (`self.ChangeAbility` (`self.ShadowTPAbility`)))

(fn `SpawnActorTransform`
  (params (Class :type "Actor Class Reference") (Transform :type "Transform Structure"))
  (returns (Actor :type "Actor Object Reference"))
  (bind _returnvalue (`|SpawnActorFromClass` Class Transform "Undefined" "MultiplyWithRoot" null null))
  (return _returnvalue))