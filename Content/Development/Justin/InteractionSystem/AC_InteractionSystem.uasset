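; Actor component that lets the player detect and interact with objects in front of the camera through BPI_Interactable.
; Each tick it sphere-traces along the camera view and switches show/hide messages as the focused interactable changes.
; An E debug key sends interact-started and interact-ended messages to that actor.
; Focus clears only when the trace hits nothing, also ending any held interaction.
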(event EventBeginPlay
  (Variables|Manager|SetCameraManager (Game|GetPlayerCameraManager 0)))

(event EventTick
  (params (DeltaSeconds :type Float%20%28single-precision%29))
  (bind _cameramanager (Variables|Manager|GetCameraManager))
  (bind _returnvalue (Camera|GetCameraLocation _cameramanager))
  ;[0.15 0.15 0.15 0.5] Scan for Interatables
  (bind (_outhit _returnvalue_2) (Collision|SphereTraceByChannel _returnvalue (+ _returnvalue (* (Math|Vector|GetForwardVector (Camera|GetCameraRotation _cameramanager)) (Variables|Interaction|GetInteractionLength))) (Variables|Interaction|GetSphereRadius) "TraceTypeQuery3" false 0 "None"))
  (if _returnvalue_2
    ;[0.15 0.15 0.15 0.5] Does object implement interface
    (if (Utilities|DoesObjectImplementInterface (.HitActor (Collision|BreakHitResult _outhit)) "/Game/Development/Justin/Interface/BPI_Interactable.BPI_Interactable_C")
      ;[0.15 0.15 0.15 0.5] Check for not equal interactable
      (if (!= (Variables|Interaction|GetInteractableActor) (.HitActor (Collision|BreakHitResult _outhit)))
        ;[0.15 0.15 0.15 0.5] Hide interaction from old interactable
        (Class|BPIInteractable|HideInteraction(Message) (Variables|Interaction|GetInteractableActor))
        ;[0.15 0.15 0.15 0.5] Show interaction by new one
        (bind _output_get (Variables|Interaction|SetInteractableActor (.HitActor (Collision|BreakHitResult _outhit))))
        (Class|BPIInteractable|ShowInteraction(Message) _output_get)))
    (else
      ;[0.15 0.15 0.15 0.5] Hide interaction
      (Utilities|IsValid (Variables|Interaction|GetInteractableActor)
        (:Is%20Valid
          (Class|BPIInteractable|HideInteraction(Message) (Variables|Interaction|GetInteractableActor))
          ;[0.15 0.15 0.15 0.5] Set interatable object in valid
          (if (Variables|Default|GetPressedInteraction)
            (Class|BPIInteractable|InteractEnded(Message) (Variables|Interaction|GetInteractableActor)))
          (Variables|Interaction|SetInteractableActor 0))))))

(event Input|KeyboardEvents|DebugKeyE
  (params (Key :type Key%20Structure :default "None") (ActionValue :type Input%20Action%20Value%20Structure))
  (:Pressed
    ;[0.15 0.15 0.15 0.5] Check if interactable actor exists
    (Utilities|IsValid (Variables|Interaction|GetInteractableActor)
      (:Is%20Valid
        ;[0.15 0.15 0.15 0.5] Start interaction
        (Variables|Default|SetPressedInteraction true)
        (Class|BPIInteractable|InteractStarted(Message) (Variables|Interaction|GetInteractableActor)))))
  (:Released
    ;[0.15 0.15 0.15 0.5] Check if interaction was valid
    (if (Variables|Default|GetPressedInteraction)
      ;[0.15 0.15 0.15 0.5] End interaction
      (Variables|Default|SetPressedInteraction false)
      (Class|BPIInteractable|InteractEnded(Message) (Variables|Interaction|GetInteractableActor)))))