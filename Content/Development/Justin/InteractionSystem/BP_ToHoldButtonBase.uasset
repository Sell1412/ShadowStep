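; Base Blueprint for hold-to-interact buttons that succeed after an interaction is held for HoldTime.
; Starting an interaction sets a timer that disables further interaction and calls OnInteractionSuccess, while ending it early clears the timer.
; OnInteractionSuccess only prints a placeholder message, apparently for children to override.
; GetHoldTimeProgress converts the timer's elapsed time into a clamped fraction of the hold duration.
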(event `/Game/Development/Justin/Interface/BPI_Interactable.InteractStarted`
  ; Interaction Started
  (if (`self.IsInteractable`)
    (bind _returnvalue (`KismetSystemLibrary.K2_SetTimerDelegate` (delegate `InteractionWorked`) (`self.HoldTime`)))
    (set `self.TimeHandler` _returnvalue)))

(event `InteractionWorked`
  (set `self.IsInteractable` false)
  (`self.OnInteractionSuccess`))

(event `/Game/Development/Justin/Interface/BPI_Interactable.InteractEnded`
  ; On Interaction End
  (if (`self.IsInteractable`)
    (`KismetSystemLibrary.K2_ClearAndInvalidateTimerHandle` (`self.TimeHandler`))
    (set `self.TimeHandler` (struct))))

(fn `GetHoldTimeProgress`
  (returns (HoldTimeProgress :type "Float (double-precision)"))
  (locals (ElapsedTime :type "Float (single-precision)" :default 0.0))
  (set `local.ElapsedTime` (`KismetSystemLibrary.K2_GetTimerElapsedTimeHandle` (`self.TimeHandler`)))
  (if (<= (`local.ElapsedTime`) 0.0)
    (return (`local.ElapsedTime`))
    (else
      (return (`KismetMathLibrary.FClamp` (/ (`local.ElapsedTime`) (`self.HoldTime`)))))))

(fn `OnInteractionSuccess`
  (`KismetSystemLibrary.PrintString` (`KismetStringLibrary.Concat_StrStr` (`KismetSystemLibrary.GetDisplayName` self) " Interaction on Success no function")))

(fn `UserConstructionScript`)