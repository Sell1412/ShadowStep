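; Actor component that manages the owner's mana in a light-and-shadow mechanic, draining it in lamp light and restoring it in moonlight shadow.
; Each tick it finds nearby BPI_ShadowTarget lights and line-traces from any within attenuation range to the player's feet, subtracting mana if unblocked.
; Otherwise, a trace from the feet against the DirectionalLight's direction detects shadow and adds mana.
; It also answers whether an ability's cost is affordable.
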(event `self.ReceiveBeginPlay`
  (set `self.CurrentManaPoints` (`self.MaxManaPoints`))
  (bind _returnvalue (`GameplayStatics.GetActorOfClass` "/Script/Engine.DirectionalLight"))
  (set `self.MoonLightDirection` (`Actor.GetActorForwardVector` _returnvalue))
  (set `self.PlayerHalfHeight` (`CapsuleComponent.CapsuleHalfHeight` (`Actor.GetComponentByClass` (`self.GetOwner`) "/Script/Engine.CapsuleComponent"))))

(event `self.ReceiveTick`
  (params (DeltaSeconds :type "Float (single-precision)"))
  ; In light sight
  (bind _inlightsight (`self.IsInLightSight`))
  (if _inlightsight
    (`self.SubtractMana` (`self.LightDamage`))
    (else
      ; In shadow logic
      (bind _newparam (`self.IsInShadow`))
      (if _newparam
        (`self.AddMana` (`self.ShadowHeal`))))))

(fn `AddMana`
  (params (ManaAmount :type "Float (double-precision)"))
  (bind _returnvalue (+ ManaAmount (`self.CurrentManaPoints`)))
  (if (<= _returnvalue (`self.MaxManaPoints`))
    (set `self.CurrentManaPoints` _returnvalue)
    (else
      (set `self.CurrentManaPoints` (`self.MaxManaPoints`))))
  (return))

(fn `IsInLightSight`
  (returns (InLightSight :type Boolean))
  (locals (CurrentPointLight :type "PointLightComponent Object Reference") (InLight :type Boolean))
  (bind _returnvalue (- (`Actor.K2_GetActorLocation` (`self.GetOwner`)) (`KismetMathLibrary.MakeVector` 0.0 0.0 (`self.PlayerHalfHeight`))))
  (set `local.InLight` false)
  (bind (_outactors _returnvalue_2) (`KismetSystemLibrary.SphereOverlapActors` (`Actor.K2_GetActorLocation` (`self.GetOwner`)) (`self.ToCheckLightRadius`) (`|MakeArray` "ObjectTypeQuery1" :!type "EObjectTypeQuery Enum")))
  (if _returnvalue_2
    (for _array_element _outactors
      (if (`KismetSystemLibrary.DoesImplementInterface` _array_element "/Game/Development/Justin/Interface/BPI_ShadowTarget.BPI_ShadowTarget_C")
        (bind _postion (message `/Game/Development/Justin/Interface/BPI_ShadowTarget.LightPostion` _array_element))
        (bind _radius (message `/Game/Development/Justin/Interface/BPI_ShadowTarget.AttentuationRaidius` _array_element))
        (if (<= (`KismetMathLibrary.Vector_Distance` _postion _returnvalue) _radius)
          (bind (_outhit _returnvalue_3) (`KismetSystemLibrary.LineTraceSingle` _postion _returnvalue "TraceTypeQuery1"))
          (if (not _returnvalue_3)
            (set `local.InLight` true)
            (break)))))
    (return (`local.InLight`))))

(fn `IsInShadow`
  (returns (NewParam :type Boolean))
  (bind _returnvalue (- (`Actor.K2_GetActorLocation` (`self.GetOwner`)) (`KismetMathLibrary.MakeVector` 0.0 0.0 (`self.PlayerHalfHeight`))))
  (bind (_outhit _returnvalue_2) (`KismetSystemLibrary.LineTraceSingle` :`Start` _returnvalue :`End` (+ _returnvalue (* (`KismetMathLibrary.NegateVector` (`self.MoonLightDirection`)) (`self.MoonLightShadowCheckLength`))) :`TraceChannel` "TraceTypeQuery1" :`DrawTime` 2.0))
  (if _returnvalue_2
    (return true)
    (else
      (return false))))

(fn `RequestAbilityUseage`
  (params (ManaCost :type "Float (double-precision)"))
  (returns (AbilityUsable :type Boolean))
  (if (< ManaCost (`self.CurrentManaPoints`))
    (return true)
    (else
      (return false))))

(fn `SubtractMana`
  (params (ManaAmount :type "Float (double-precision)"))
  (bind _returnvalue (- (`self.CurrentManaPoints`) ManaAmount))
  (if (>= _returnvalue 0.0)
    (set `self.CurrentManaPoints` _returnvalue)
    (return)))