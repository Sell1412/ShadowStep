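; Actor component that manages the player's shadow abilities, holding a shadow teleport ability and a light ability as separate objects.
; It constructs and initialises both on BeginPlay, then forwards Tick and teleport input press and release to the current ability.
; Debug keys switch between them, deactivating the outgoing ability first.
; Helpers for camera, directional light and indicator setup remain, but their setup chain is disconnected.
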(event Input|EnhancedActionEvents|EnhancedInputActionIA_Teleport
  (params (ActionValue :type Boolean) (ElapsedSeconds :type Float%20%28double-precision%29) (TriggeredSeconds :type Float%20%28double-precision%29) (InputAction :type Input%20Action%20Object%20Reference :default "/Game/Development/Tobias/ThirdPerson/Input/Actions/IA_Teleport.IA_Teleport"))
  (bind _currentability (Variables|CurrentAbility|GetCurrentAbility))
  (:Started
    (Default|Started _currentability))
  (:Canceled
    (Default|Released _currentability :!label _label))
  (:Completed
    (goto _label)))

(event EventBeginPlay
  (bind _returnvalue (Game|ConstructObjectfromClass "/Game/Development/Justin/Abilitys/Teleport/O_ShadowAbility_TP.O_ShadowAbility_TP_C"))
  (bind _output_get (Variables|Ability|SetShadowAbility _returnvalue))
  (Default|Initialise _output_get self)
  (bind _returnvalue_2 (Game|ConstructObjectfromClass "/Game/Development/Justin/DataAssets/O_ShadowAbility_Light.O_ShadowAbility_Light_C"))
  (bind _output_get_2 (Variables|Ability|SetLightAbility _returnvalue_2))
  (Default|Initialise _output_get_2 self))

(event EventTick
  (params (DeltaSeconds :type Float%20%28single-precision%29))
  (Default|Tick (Variables|CurrentAbility|GetCurrentAbility)))

(event Input|KeyboardEvents|DebugKey1
  (params (Key :type Key%20Structure :default "None") (ActionValue :type Input%20Action%20Value%20Structure))
  (:Pressed
    (CallFunction|ChangeAbility (Variables|Ability|GetShadowAbility))))

(event Input|KeyboardEvents|DebugKey2
  (params (Key :type Key%20Structure :default "None") (ActionValue :type Input%20Action%20Value%20Structure))
  (:Pressed
    (CallFunction|ChangeAbility (Variables|Ability|GetLightAbility))))

(fn SpawnActor
  (params (Class :type Actor%20Class%20Reference) (Loaction :type Vector))
  (bind _returnvalue (Game|SpawnActorfromClass Class (Math|Transform|MakeTransform Loaction) "Undefined" "MultiplyWithRoot" 0 0))
  (return _returnvalue))

(fn ChangeAbility
  (params (NewAblity :type O%20Shadow%20Ability%20Base%20Object%20Reference))
  (Default|OnAbilityDeactivated (Variables|CurrentAbility|GetCurrentAbility))
  (Variables|CurrentAbility|SetCurrentAbility NewAblity))