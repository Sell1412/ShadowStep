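; Player actor component that lets the player execute nearby enemies.
; It maintains a unique list of nearby enemies through add and remove functions, each firing a matching event dispatcher.
; A debug E key press kills the first listed enemy via its AI health component, disables its execute box, and reports a noise event at the owner's location within a set range.
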(event EventBeginPlay)

(event EventTick
  (params (DeltaSeconds :type Float%20%28single-precision%29)))

(event Input|KeyboardEvents|DebugKeyE
  (params (Key :type Key%20Structure :default "None") (ActionValue :type Input%20Action%20Value%20Structure))
  (bind _returnvalue (Components|GetOwner))
  (:Pressed
    (if (|NearbyEnemyList>0)
      (CallFunction|ExecuteEnemy (Utilities|Array|Get(acopy) (Variables|Default|GetNearbyEnemys)))
      ;[0.15 0.15 0.15 0.5] MakeSound
      (Class|AISenseHearing|ReportNoiseEvent (Transformation|GetActorLocation _returnvalue) 1.0 _returnvalue (Variables|Default|GetKillNoiceSoundRange) "None"))))

(fn AddNearbyEnemy
  (params (New%20Enemy :type BP%20Enemy%20Base%20Object%20Reference))
  (Utilities|Array|AddUnique (Variables|Default|GetNearbyEnemys) New%20Enemy)
  (Default|CallOnEnemyAdded New%20Enemy))

(fn RemoveNearbyEnemy
  (params (Removing%20Enemy :type BP%20Enemy%20Base%20Object%20Reference))
  (bind _returnvalue (Utilities|Array|RemoveItem (Variables|Default|GetNearbyEnemys) Removing%20Enemy))
  (if _returnvalue
    (Default|CallOnEnemyRemove Removing%20Enemy)))

(fn ExecuteEnemy
  (params (ToKilEnemy :type BP%20Enemy%20Base%20Object%20Reference))
  (Utilities|IsValid ToKilEnemy
    (:Is%20Valid
      (Development|PrintString "KILL ENEMY")
      (Development|PrintString (Utilities|GetDisplayName ToKilEnemy))
      (Default|OnDeath (Variables|/Game/Development/Tobias/Blueprints/Enemy/Core/BP_EnemyBase.BP_EnemyBase_C|GetAC_AIHealth ToKilEnemy))
      (Default|DisableExecuteBox ToKilEnemy))))