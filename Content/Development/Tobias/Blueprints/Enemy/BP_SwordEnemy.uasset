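; BP_SwordEnemy is a sword enemy Blueprint whose own logic handles being alerted by its group.
; GetNotified, if the enemy is alive and not yet notified, writes the group-notified flag, chase state, chase time and player location to the Blackboard.
; It then maxes suspicion through AIC_BaseController.
; Blackboard writes use the Owner's AI controller, while the suspicion call uses the enemy's own.
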(fn `GetNotified`
  (locals (ChaseState :type "/Game/Development/Tobias/Blueprints/Enemy/Core/Enum/E_EnemyState Enum" :default "NewEnumerator2"))
  (bind _returnvalue (`AIBlueprintHelperLibrary.GetAIController` (`self.GetOwner`)))
  (bind _blackboard (`AIController.Blackboard` _returnvalue))
  ; Onlfy if enemy is Alive
  (if (`/Game/Development/Tobias/Blueprints/Enemy/Core/Component/AC_AIHealth.IsDead` (`self.AC_AIHealth`))
    _
    (elif (not (`self.IsNotified`))
      (`/Engine/EditorBlueprintResources/StandardMacros.IsValid` _returnvalue
        (:`Is Valid`
          (`BlackboardComponent.SetValueAsBool` _blackboard "HasBeenNotifiedByGroup" true)
          ; Set Chase State
          (`BlackboardComponent.SetValueAsEnum` _blackboard "EnemyState" (`local.ChaseState`))
          ; Set Chase Time
          (`BlackboardComponent.SetValueAsFloat` _blackboard "RemaingChaseTime" (`BlackboardComponent.GetValueAsFloat` _blackboard "ChaseTime"))
          ; Set Target Actor
          (`BlackboardComponent.SetValueAsVector` _blackboard "CheckingLocation" (`self.K2_GetActorLocation` (`GameplayStatics.GetPlayerCharacter` 0)))
          (bind _asaic_base_controller (cast `/Game/Development/Tobias/Blueprints/Enemy/Core/AI/AIC_BaseController` (`AIBlueprintHelperLibrary.GetAIController` self)))
          (`/Game/Development/Tobias/Blueprints/Enemy/Core/AI/AIC_BaseController.SetSusFull` _asaic_base_controller))))))

(fn `UserConstructionScript`
  (`parent.UserConstructionScript`))