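; AC_BackstabComponent is an enemy actor component that reports whether its owner can be backstabbed.
; IsBackstabable gets the owner's AI controller as AIC_BaseController and returns false if its EnemyState matches one specific value or its HealthComponent reports dead.
; Otherwise it returns true; the component has no active event logic.
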(fn `IsBackstabable`
  (returns (CanBeBackstabed :type Boolean))
  (bind _asaic_base_controller (cast `/Game/Development/Tobias/Blueprints/Enemy/Core/AI/AIC_BaseController` (`AIBlueprintHelperLibrary.GetAIController` (`self.GetOwner`))))
  (if (`|EnumEquality` (`/Game/Development/Tobias/Blueprints/Enemy/Core/AI/AIC_BaseController.EnemyState` _asaic_base_controller) "NewEnumerator2")
    (return false)
    (elif (`/Game/Development/Tobias/Blueprints/Enemy/Core/Component/AC_AIHealth.IsDead` (`/Game/Development/Tobias/Blueprints/Enemy/Core/AI/AIC_BaseController.HealthComponent` _asaic_base_controller))
      (return false)
      (else
        (return true)))))