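; Enemy AI health component that handles death and reset for BP_EnemyBase characters.
; OnDeath switches the mesh to ragdoll physics with a random impulse, disables capsule collision, broadcasts OnEnemyDeath and flags IsDead.
; Reset undoes the ragdoll, restoring collision, the unarmed anim instance and mesh offset, then clears IsDead.
; A separate SetDead function writes the IsDead key to the owner's AI blackboard.
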(event `self.ReceiveBeginPlay`)

(event `OnDeath`
  (`self.EnableRagdoll`)
  (`self.OnEnemyDeath`)
  ; Sound
  (set `self.IsDead` true))

(fn `DisableRagdoll`
  (bind _asbp_enemy_base (cast `/Game/Development/Tobias/Blueprints/Enemy/Core/BP_EnemyBase` (`self.GetOwner`)))
  (bind _mesh (`Character.Mesh` _asbp_enemy_base))
  (`PrimitiveComponent.SetCollisionProfileName` _mesh "Enemy" true)
  (`SkeletalMeshComponent.SetAllBodiesSimulatePhysics` _mesh false)
  (`PrimitiveComponent.SetCollisionEnabled` (`Character.CapsuleComponent` _asbp_enemy_base) "QueryAndPhysics")
  (`SkeletalMeshComponent.SetAnimInstanceClass` _mesh "/Game/Development/Tobias/ThirdPerson/Mannequins/Anims/Unarmed/ABP_Unarmed.ABP_Unarmed_C")
  (`SceneComponent.K2_SetRelativeRotation` _mesh (struct :`Yaw` -90.0) false false)
  (`SceneComponent.K2_SetRelativeLocation` _mesh (0.0 0.0 -80.0) false false))

(fn `EnableRagdoll`
  (locals (Mesh :type "SkeletalMeshComponent Object Reference"))
  (bind _asbp_enemy_base (cast `/Game/Development/Tobias/Blueprints/Enemy/Core/BP_EnemyBase` (`self.GetOwner`)))
  (bind _output_get (set `local.Mesh` (`Character.Mesh` _asbp_enemy_base)))
  (`PrimitiveComponent.SetCollisionProfileName` _output_get "Ragdoll" true)
  (`SkeletalMeshComponent.SetAllBodiesSimulatePhysics` (`local.Mesh`) true)
  (`PrimitiveComponent.SetCollisionEnabled` (`Character.CapsuleComponent` _asbp_enemy_base) "NoCollision")
  (`PrimitiveComponent.AddImpulse` (`local.Mesh`) (`KismetMathLibrary.RandomUnitVector`) "None" false))

(fn `Reset`
  (`self.DisableRagdoll`)
  (set `self.IsDead` false))

(fn `SetDead`
  (params (BoolValue :type Boolean))
  (`BlackboardComponent.SetValueAsBool` (`AIBlueprintHelperLibrary.GetBlackboard` (`AIBlueprintHelperLibrary.GetAIController` (`self.GetOwner`))) "IsDead" BoolValue))