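; Base enemy Blueprint that configures its AI, health and backstab execution, and resets with the world.
; BeginPlay pushes its tuning values into the health and AI components, AIC_BaseController, blackboard and sight settings, then binds alert, death and world-reset events.
; An overlap box registers backstabable enemies with the player's execute component, while a suspicion widget rotates toward the camera each tick.
; World reset restores state and teleports it to its spawn transform.
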(event `OnAlertEnd`
  (set `/Game/Development/Tobias/Blueprints/Enemy/Core/AI/AIC_BaseController.IsAlerted` false (`self.OwnAIController`)))

(event `OnAlertStart`
  (set `/Game/Development/Tobias/Blueprints/Enemy/Core/AI/AIC_BaseController.IsAlerted` true (`self.OwnAIController`)))

(event `OnWorldReset_Event`
  (bind (_spawntransform_location _spawntransform_rotation) (`KismetMathLibrary.BreakTransform` (`self.SpawnTransform`)))
  (`self.Reset`)
  (`self.K2_TeleportTo` _spawntransform_location _spawntransform_rotation))

(event `OnEnemyDeath_Event`
  (`self.SetDeathValues`))

(event `self.ReceiveBeginPlay`
  (bind _isdead (`self.IsDead`))
  (bind _ac_aihealth (`self.AC_AIHealth`))
  (bind _returnvalue (`AIBlueprintHelperLibrary.GetAIController` self))
  (bind _aswbp_sus_infos (cast `/Game/Development/Tobias/Blueprints/Enemy/Core/Widget/WBP_SusInfos` (`WidgetComponent.GetWidget` (`self.SusWidget`))))
  (set `/Game/Development/Tobias/Blueprints/Enemy/Core/Widget/WBP_SusInfos.Owner` self _aswbp_sus_infos)
  (`|ExecutionSequence`
    (:`then_0`
      (`/Game/Development/Tobias/Blueprints/Enemy/Core/Component/AC_AIHealth.SetDead` _ac_aihealth _isdead)
      (if _isdead
        (`/Game/Development/Tobias/Blueprints/Enemy/Core/Component/AC_AIHealth.OnDeath` _ac_aihealth)))
    (:`then_1`
      (`/Game/Development/Tobias/Blueprints/Enemy/Core/Component/AC_AIComponent.SetStartState` (`self.AC_AIComponent`) (`self.StartState`))
      (set `/Game/Development/Tobias/Blueprints/Enemy/Core/Component/AC_AIComponent.PatrolMovementSpeed` (`self.PatrolSpeed`) (`self.AC_AIComponent`))
      (set `/Game/Development/Tobias/Blueprints/Enemy/Core/Component/AC_AIComponent.SearchMovementSpeed` (`self.SearchSpeed`) (`self.AC_AIComponent`))
      (set `/Game/Development/Tobias/Blueprints/Enemy/Core/Component/AC_AIComponent.ChaseMovementSpeed` (`self.ChaseSpeed`) (`self.AC_AIComponent`))
      (bind _output_get (set `/Game/Development/Tobias/Blueprints/Enemy/Core/Component/AC_AIComponent.PatrolPoints` (`self.Patrol Points`) (`self.AC_AIComponent`)))
      (`BlackboardComponent.SetValueAsBool` (`AIBlueprintHelperLibrary.GetBlackboard` (`AIBlueprintHelperLibrary.GetAIController` self)) "HasPatrolPoints" (> (`BlueprintMapLibrary.Map_Length` _output_get) 0)))
    (:`then_2`
      (bind _asaic_base_controller (cast `/Game/Development/Tobias/Blueprints/Enemy/Core/AI/AIC_BaseController` (`AIBlueprintHelperLibrary.GetAIController` self)))
      (bind _output_get_2 (set `self.OwnAIController` _asaic_base_controller))
      (set `/Game/Development/Tobias/Blueprints/Enemy/Core/AI/AIC_BaseController.UpdateSusInterval` (`self.Update Sus Interval`) _output_get_2)
      (set `/Game/Development/Tobias/Blueprints/Enemy/Core/AI/AIC_BaseController.AlertedTime` (`self.Alerted Time`) (`self.OwnAIController`))
      (set `/Game/Development/Tobias/Blueprints/Enemy/Core/AI/AIC_BaseController.FillRates` (`self.Fill Rates`) (`self.OwnAIController`))
      (set `/Game/Development/Tobias/Blueprints/Enemy/Core/AI/AIC_BaseController.Debug Sphere` (`self.Notify Debug Sphere`) (`self.OwnAIController`)))
    (:`then_3`
      (`AISenseLibary.SetSightRange` _returnvalue (`self.SightRange`))
      (`AISenseLibary.SetSightAngle` _returnvalue (`self.Sight Angle`))
      (`|ExecutionSequence`
        (:`then_0`
          (bind _asaic_base_controller_2 (cast `/Game/Development/Tobias/Blueprints/Enemy/Core/AI/AIC_BaseController` (`AIBlueprintHelperLibrary.GetAIController` self)))
          (add `/Game/Development/Tobias/Blueprints/Enemy/Core/AI/AIC_BaseController.OnAlertEnd` _asaic_base_controller_2 (delegate `OnAlertEnd`))
          (add `/Game/Development/Tobias/Blueprints/Enemy/Core/AI/AIC_BaseController.OnAlertStart` _asaic_base_controller_2 (delegate `OnAlertStart`)))
        (:`then_1`
          (bind _asbp_world_game_mode (cast `/Game/ShadowStep/Core/ProjectManagers/BP_WorldGameMode` (`GameplayStatics.GetGameMode`)))
          (add `/Game/ShadowStep/Core/ProjectManagers/BP_WorldGameMode.OnWorldReset` _asbp_world_game_mode (delegate `OnWorldReset_Event`)))
        (:`then_2`
          (add `/Game/Development/Tobias/Blueprints/Enemy/Core/Component/AC_AIHealth.OnEnemyDeath` (`self.AC_AIHealth`) (delegate `OnEnemyDeath_Event`)))))
    (:`then_4`
      (`BlackboardComponent.SetValueAsFloat` (`AIBlueprintHelperLibrary.GetBlackboard` (`AIBlueprintHelperLibrary.GetAIController` self)) "ChaseTime" (`self.Chase Time`)))
    (:`then_5`
      (set `self.SpawnTransform` (`self.GetTransform`)))))

(event `self.ReceiveTick`
  (params (DeltaSeconds :type "Float (single-precision)"))
  (`self.RotateWidgetToCamera` (`self.SusWidget`)))

(event `self.ExecuteBox.OnComponentBeginOverlap`
  (params (OverlappedComponent :type "PrimitiveComponent Object Reference") (OtherActor :type "Actor Object Reference") (OtherComp :type "PrimitiveComponent Object Reference") (OtherBodyIndex :type Integer) (bFromSweep :type Boolean) (SweepResult :type "HitResult Structure (by ref)"))
  (bind _returnvalue (`GameplayStatics.GetPlayerCharacter` 0))
  (bind _returnvalue_2 (`self.GetComponentByClass` _returnvalue "/Game/Development/Tobias/Blueprints/Player/Component/AC_ExecuteComponent.AC_ExecuteComponent_C"))
  (if (== OtherActor _returnvalue)
    (bind _canbebackstabed (`/Game/Development/Tobias/Blueprints/Enemy/Core/Component/AC_BackstabComponent.IsBackstabable` (`self.AC_BackstabComponent`)))
    (if _canbebackstabed
      (`/Engine/EditorBlueprintResources/StandardMacros.IsValid` _returnvalue_2
        (:`Is Valid`
          (`/Game/Development/Tobias/Blueprints/Player/Component/AC_ExecuteComponent.AddNearbyEnemy` _returnvalue_2 self))))))

(event `self.ExecuteBox.OnComponentEndOverlap`
  (params (OverlappedComponent :type "PrimitiveComponent Object Reference") (OtherActor :type "Actor Object Reference") (OtherComp :type "PrimitiveComponent Object Reference") (OtherBodyIndex :type Integer))
  (bind _returnvalue (`GameplayStatics.GetPlayerCharacter` 0))
  (bind _returnvalue_2 (`self.GetComponentByClass` _returnvalue "/Game/Development/Tobias/Blueprints/Player/Component/AC_ExecuteComponent.AC_ExecuteComponent_C"))
  (if (== OtherActor _returnvalue)
    (`/Engine/EditorBlueprintResources/StandardMacros.IsValid` _returnvalue_2
      (:`Is Valid`
        (`/Game/Development/Tobias/Blueprints/Player/Component/AC_ExecuteComponent.RemoveNearbyEnemy` _returnvalue_2 self)))))

(fn `DisableExecuteBox`
  (`PrimitiveComponent.SetCollisionEnabled` (`self.ExecuteBox`) "NoCollision"))

(fn `EnablleExecuteBox`
  (`PrimitiveComponent.SetCollisionEnabled` (`self.ExecuteBox`) "QueryOnly"))

(fn `GetNotified`
  (return))

(fn `Reset`
  (`/Game/Development/Tobias/Blueprints/Enemy/Core/Component/AC_AIHealth.Reset` (`self.AC_AIHealth`))
  (`/Game/Development/Tobias/Blueprints/Enemy/Core/Component/AC_AIComponent.Reset` (`self.AC_AIComponent`))
  (`/Game/Development/Tobias/Blueprints/Enemy/Core/AI/AIC_BaseController.Reset` (`self.OwnAIController`))
  (`/Game/Development/Tobias/Blueprints/AreaControl/AC_AreaControl.DeactivateArea` (`self.AC_AreaControl`))
  ; Own Values
  (set `self.IsDead` false)
  (set `self.IsNotified` false)
  (`self.EnablleExecuteBox`))

(fn `RotateWidgetToCamera`
  (params (Widget :type "WidgetComponent Object Reference"))
  (`SceneComponent.K2_SetWorldRotation` Widget (`KismetMathLibrary.FindLookAtRotation` (`SceneComponent.K2_GetComponentLocation` Widget) (`PlayerCameraManager.GetCameraLocation` (`PlayerController.PlayerCameraManager` (`GameplayStatics.GetPlayerController` 0)))) false false))

(fn `SetDeathValues`
  (`/Game/Development/Tobias/Blueprints/Enemy/Core/AI/AIC_BaseController.SetDeathValues` (`self.OwnAIController`)))

(fn `UserConstructionScript`)