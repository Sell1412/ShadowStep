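; BP_Checkpoint is a respawn checkpoint that registers itself when the player character enters its area trigger.
; The overlap passes the checkpoint to BP_WorldGameMode as the new checkpoint and, if flagged to load a new area, calls OnNewAreaLoad with itself.
; GetRespawnLocation returns the world transform of its RespawnPoint component for placing the respawned player.
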(event `self.ReceiveBeginPlay`
  (bind _asbp_world_game_mode (cast `/Game/ShadowStep/Core/ProjectManagers/BP_WorldGameMode` (`GameplayStatics.GetGameMode`)))
  (set `self.Gamemode` _asbp_world_game_mode))

(event `self.EnterAreaTrigger.OnComponentBeginOverlap`
  (params (OverlappedComponent :type "PrimitiveComponent Object Reference") (OtherActor :type "Actor Object Reference") (OtherComp :type "PrimitiveComponent Object Reference") (OtherBodyIndex :type Integer) (bFromSweep :type Boolean) (SweepResult :type "HitResult Structure (by ref)"))
  ; Player enters Area
  (cast `/Game/ShadowStep/Characters/Player/BP_PlayerCharakter` OtherActor)
  (`self.SetNewCheckpoint`)
  (if (`self.bShouldLoadNewArea`)
    (`self.OnNewAreaLoad` self)))

(fn `GetRespawnLocation`
  (returns (RespawnLocation :type "Transform Structure"))
  (return (`SceneComponent.K2_GetComponentToWorld` (`self.RespawnPoint`))))

(fn `SetNewCheckpoint`
  (bind _asbp_world_game_mode (cast `/Game/ShadowStep/Core/ProjectManagers/BP_WorldGameMode` (`GameplayStatics.GetGameMode`)))
  (bind _sucessfull (`/Game/ShadowStep/Core/ProjectManagers/BP_WorldGameMode.SetNewCheckpoint` _asbp_world_game_mode self))
  (if _sucessfull
    _))

(fn `UserConstructionScript`)