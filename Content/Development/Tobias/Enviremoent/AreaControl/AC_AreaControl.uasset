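; AC_AreaControl is an actor component that switches its owning AI-controlled actor on or off, apparently for area-based activation.
; ActivateArea starts the brain component logic on the owner's AI controller and enables the owner's actor tick.
; DeactivateArea stops that logic and disables the tick.
; The component has no active event logic, so both functions depend on external callers.
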(fn `ActivateArea`
  (`BrainComponent.StartLogic` (`AIController.BrainComponent` (`AIBlueprintHelperLibrary.GetAIController` (`self.GetOwner`))))
  (`Actor.SetActorTickEnabled` (`self.GetOwner`) true))

(fn `DeactivateArea`
  (`BrainComponent.StopLogic` (`AIController.BrainComponent` (`AIBlueprintHelperLibrary.GetAIController` (`self.GetOwner`))) "")
  (`Actor.SetActorTickEnabled` (`self.GetOwner`) false))